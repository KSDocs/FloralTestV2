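; BP_Explosion is a one-shot explosion actor that pushes and damages its surroundings when spawned.
; On BeginPlay, its outer and inner radial force components fire impulses, and their radii also size two radial damage calls centered on the inner component.
; Outer damage falls off with distance while inner damage applies in full, so the two stack near the core.
; The actor then expires after a short lifespan.
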(event EventBeginPlay
  (bind _innerexplosion (Variables|Default|GetInnerExplosion))
  (Class|RadialForceComponent|FireImpulse (Variables|Default|GetOuterExplosion))
  ;[1 1 1] OuterCore Damage
  (Game|Damage|ApplyRadialDamage (Variables|Default|GetOuterDamage) (Transformation|GetWorldLocation (Variables|Default|GetInnerExplosion)) (Variables|/Script/Engine.RadialForceComponent|GetRadius (Variables|Default|GetOuterExplosion)) 0 0 0 0 false "ECC_Visibility")
  ;[1 1 1] InnerCore Damage
  (Game|Damage|ApplyRadialDamage (Variables|Default|GetInnerDamage) (Transformation|GetWorldLocation _innerexplosion) (Variables|/Script/Engine.RadialForceComponent|GetRadius _innerexplosion) 0 0 0 0 true "ECC_Visibility")
  (Actor|SetLifeSpan 3.0))

(fn ConstructionScript)